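; Armored skeleton enemy that faces player 0, damages and stuns Kaelan on contact, then briefly rebounds.
; Construction script sockets armor pieces onto the mesh.
; Hammer overlaps drop helmet, then chestplate as short-lived physics debris, granting brief invincibility and stun; with no armor left, it dies and credits the Hammer's kills and score.
; Stun skips parent Tick and turning, and also triggers on hits from other non-WorldStatic objects.
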(event `self.ReceiveBeginPlay`
  (`parent.ReceiveBeginPlay`))

(event `self.ReceiveTick`
  (params (DeltaSeconds :type "Float (single-precision)"))
  (bind (_returnvalue_roll _returnvalue_pitch _returnvalue_yaw) (`KismetMathLibrary.BreakRotator` (`KismetMathLibrary.FindLookAtRotation` (`self.K2_GetActorLocation`) (`self.K2_GetActorLocation` (`GameplayStatics.GetPlayerCharacter` 0)))))
  (if (not (`self.Stunned`))
    (if (not (`self.Rebounding`))
      (`self.K2_SetActorRotation` (`KismetMathLibrary.MakeRotator` 0.0 0.0 _returnvalue_yaw)))
    (`parent.ReceiveTick` DeltaSeconds)))

(event `self.CapsuleComponent.OnComponentBeginOverlap`
  (params (OverlappedComponent :type "PrimitiveComponent Object Reference") (OtherActor :type "Actor Object Reference") (OtherComp :type "PrimitiveComponent Object Reference") (OtherBodyIndex :type Integer) (bFromSweep :type Boolean) (SweepResult :type "HitResult Structure (by ref)"))
  (bind _armor (`self.Armor`))
  (bind _ashammer (cast `/Game/Blueprints/Hammer` OtherActor))
  (if (`self.InvincibilityFrame`)
    _
    (elif (== _armor 0)
      (`/Engine/EditorBlueprintResources/StandardMacros.IncrementInt` (`/Game/Blueprints/Hammer.KillCount` _ashammer)
        (:`  `
          (set `/Game/Blueprints/Hammer.KillScore` (+ (`/Game/Blueprints/Hammer.KillScore` _ashammer) (`self.ScoreValue`)) _ashammer)
          (`parent.Die`)))
      (else
        (set `self.InvincibilityFrame` true)
        (`KismetSystemLibrary.K2_SetTimerDelegate` (delegate `BecomeVulnerable`) 0.7)
        (if (== _armor 2)
          (`PrimitiveComponent.SetSimulatePhysics` (`self.Helmet`) true)
          (`/Engine/EditorBlueprintResources/StandardMacros.DecrementInt` (`self.Armor`)
            (:`  `
              (`self.Stun` 1.0)
              (`KismetSystemLibrary.K2_SetTimerDelegate` (delegate `DestroyHelmet`) 0.7)))
          (else
            (`PrimitiveComponent.SetSimulatePhysics` (`self.Chestplate`) true)
            (`/Engine/EditorBlueprintResources/StandardMacros.DecrementInt` (`self.Armor`)
              (:`  `
                (`self.Stun` 1.0)
                (`KismetSystemLibrary.K2_SetTimerDelegate` (delegate `DestroyArmor`) 0.7)))))))))

(event `DestroyHelmet`
  (`ActorComponent.K2_DestroyComponent` (`self.Helmet`)))

(event `BecomeVulnerable`
  (set `self.InvincibilityFrame` false))

(event `DestroyArmor`
  (`ActorComponent.K2_DestroyComponent` (`self.Chestplate`)))

(event `StopRebound`
  (set `self.Rebounding` false))

(event `self.CapsuleComponent.OnComponentHit`
  (params (HitComponent :type "PrimitiveComponent Object Reference") (OtherActor :type "Actor Object Reference") (OtherComp :type "PrimitiveComponent Object Reference") (NormalImpulse :type "Vector Structure") (Hit :type "HitResult Structure (by ref)"))
  (bind (_returnvalue_roll _returnvalue_pitch _returnvalue_yaw) (`KismetMathLibrary.BreakRotator` (`KismetMathLibrary.Conv_VectorToRotator` (`KismetMathLibrary.GetReflectionVector` (`KismetMathLibrary.GetDirectionUnitVector` (`self.K2_GetActorLocation`))))))
  (bind _askaelan (cast `/Game/Blueprints/Kaelan` OtherActor)
    (:`then`
      (if (not (`self.Rebounding`))
        (`/Game/Blueprints/Kaelan.Stun` _askaelan)
        (`/Game/Blueprints/Kaelan.TakeDamage` _askaelan 7.5)
        (set `self.Rebounding` true)
        (`self.K2_SetActorRotation` (`KismetMathLibrary.MakeRotator` 0.0 0.0 _returnvalue_yaw))
        (`KismetSystemLibrary.K2_SetTimerDelegate` (delegate `StopRebound`) 1.5)))
    (:`CastFailed`
      (if (`|EnumInequality` (`PrimitiveComponent.GetCollisionObjectType` (`.HitComponent` (`GameplayStatics.BreakHitResult` Hit))) "ECC_WorldStatic")
        (`self.Stun` 0.5)))))

(event `Stun`
  (params (Stuntime :type "Float (double-precision)"))
  (`KismetSystemLibrary.K2_SetTimerDelegate` (delegate `Unstun`) Stuntime)
  (set `self.Stunned` true))

(event `Unstun`
  (set `self.Stunned` false))

(fn `UserConstructionScript`
  (`parent.UserConstructionScript`)
  (`SceneComponent.K2_AttachToComponent` (`self.LeftGuard`) (`self.Mesh`) "ForearmLeft" "KeepRelative" "KeepRelative" "KeepRelative" true)
  (`SceneComponent.K2_AttachToComponent` (`self.RightGuard`) (`self.Mesh`) "ForearmRight" "KeepRelative" "KeepRelative" "KeepRelative" true)
  (`SceneComponent.K2_AttachToComponent` (`self.LeftGreave`) (`self.Mesh`) "ShinLeft" "KeepRelative" "KeepRelative" "KeepRelative" true)
  (`SceneComponent.K2_AttachToComponent` (`self.RightGreave`) (`self.Mesh`) "ShinRight" "KeepRelative" "KeepRelative" "KeepRelative" true)
  (`SceneComponent.K2_AttachToComponent` (`self.Chestplate`) (`self.Mesh`) "Torso" "KeepRelative" "KeepRelative" "KeepRelative" true)
  (`SceneComponent.K2_AttachToComponent` (`self.Helmet`) (`self.Mesh`) "Head" "KeepRelative" "KeepRelative" "KeepRelative" true))