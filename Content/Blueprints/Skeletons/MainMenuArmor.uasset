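; Armored skeleton actor, apparently for the main menu, that removes itself after a short lifetime.
; The construction script runs the parent's, then attaches forearm guards, greaves, chestplate and helmet to named sockets on the Mesh, keeping relative transforms.
; BeginPlay sets a fixed half-turn rotation and starts a one-shot timer that destroys the actor after 20 seconds.
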(event `Die`
  (`self.K2_DestroyActor`))

(event `self.ReceiveBeginPlay`
  (`self.K2_SetActorRotation` (struct :`Yaw` 180.0))
  (`KismetSystemLibrary.K2_SetTimerDelegate` (delegate `Die`) 20.0))

(fn `UserConstructionScript`
  (`parent.UserConstructionScript`)
  (`SceneComponent.K2_AttachToComponent` (`self.LeftGuard`) (`self.Mesh`) "ForearmLeft" "KeepRelative" "KeepRelative" "KeepRelative" true)
  (`SceneComponent.K2_AttachToComponent` (`self.RightGuard`) (`self.Mesh`) "ForearmRight" "KeepRelative" "KeepRelative" "KeepRelative" true)
  (`SceneComponent.K2_AttachToComponent` (`self.LeftGreave`) (`self.Mesh`) "ShinLeft" "KeepRelative" "KeepRelative" "KeepRelative" true)
  (`SceneComponent.K2_AttachToComponent` (`self.RightGreave`) (`self.Mesh`) "ShinRight" "KeepRelative" "KeepRelative" "KeepRelative" true)
  (`SceneComponent.K2_AttachToComponent` (`self.Chestplate`) (`self.Mesh`) "Torso" "KeepRelative" "KeepRelative" "KeepRelative" true)
  (`SceneComponent.K2_AttachToComponent` (`self.Helmet`) (`self.Mesh`) "Head" "KeepRelative" "KeepRelative" "KeepRelative" true))