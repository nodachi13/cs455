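; Main menu skeleton character, apparently decorative, that walks forward on its own and cleans itself up after a short lifetime.
; BeginPlay turns it to face roughly backward along world X with a random yaw spread and gives a one-in-three chance of the poison skeleton material.
; Tick feeds forward movement input while Alive is true, and a one-shot timer calls Die to destroy the actor.
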(event `Die`
  (`self.K2_DestroyActor`))

(event `self.ReceiveBeginPlay`
  (bind _mesh (`self.Mesh`))
  (`KismetSystemLibrary.K2_SetTimerDelegate` (delegate `Die`) 15.0)
  (`self.K2_SetActorRotation` (`KismetMathLibrary.MakeRotator` 0.0 0.0 (+ (`KismetMathLibrary.RandomFloatInRange` -15.0 15.0) 180.0)))
  (if (== (`KismetMathLibrary.RandomIntegerInRange` 0 2) 0)
    (`PrimitiveComponent.SetMaterial` _mesh 0 "/Game/Assets/Materials/SkelemanPoisonMat.SkelemanPoisonMat")
    (`PrimitiveComponent.SetMaterial` _mesh 1 "/Game/Assets/Materials/SkelemanPoisonMat.SkelemanPoisonMat")))

(event `self.ReceiveTick`
  (params (DeltaSeconds :type "Float (single-precision)"))
  (if (`self.Alive`)
    (`self.AddMovementInput` (`self.GetActorForwardVector`))))

(fn `UserConstructionScript`)