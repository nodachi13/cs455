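; Short-lived poison cloud hazard that damages the Kaelan character inside it, then destroys itself after a few seconds.
; A looping timer runs a pawn sphere trace at the cloud's location and applies damage to hits that cast to Kaelan.
; The construction script builds fog-sheet dynamic materials for four meshes, tinted by Color and Brightness.
; Tick animates three of them with fixed per-frame scale changes, shrinking one and growing two.
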(event `Die`
  (`self.K2_DestroyActor`))

(event `self.ReceiveBeginPlay`
  (`KismetSystemLibrary.K2_SetTimerDelegate` (delegate `Poison`) 0.15 true)
  (`KismetSystemLibrary.K2_SetTimerDelegate` (delegate `Die`) 5.5))

(event `Poison`
  (bind _returnvalue (`self.K2_GetActorLocation`))
  (bind _outhits (`KismetSystemLibrary.SphereTraceMultiForObjects` _returnvalue _returnvalue 150.0 (`|MakeArray` "ObjectTypeQuery3" :!type "EObjectTypeQuery Enum")))
  (for _array_element _outhits
    (bind _askaelan (cast `/Game/Blueprints/Kaelan` (`.HitActor` (`GameplayStatics.BreakHitResult` _array_element))))
    (`/Game/Blueprints/Kaelan.TakeDamage` _askaelan 1.0)))

(event `self.ReceiveTick`
  (params (DeltaSeconds :type "Float (single-precision)"))
  (bind _staticmesh1 (`self.StaticMesh1`))
  (bind _staticmesh2 (`self.StaticMesh2`))
  (bind _staticmesh3 (`self.StaticMesh3`))
  (`SceneComponent.SetRelativeScale3D` _staticmesh1 (+ (`SceneComponent.RelativeScale3D` _staticmesh1) -0.005))
  (`SceneComponent.SetRelativeScale3D` _staticmesh2 (+ (`SceneComponent.RelativeScale3D` _staticmesh2) 0.0085))
  (`SceneComponent.SetRelativeScale3D` _staticmesh3 (+ (`SceneComponent.RelativeScale3D` _staticmesh3) 0.01)))

(fn `ApplyFogSheet`
  (params (FogSheetMID :type "MaterialInstanceDynamic Object Reference"))
  (bind _brightness (`self.Brightness`))
  (bind (_r _g _b _a) (`KismetMathLibrary.BreakColor` (`self.color`)))
  (`MaterialInstanceDynamic.SetVectorParameterValue` FogSheetMID "Color" (`KismetMathLibrary.MakeColor` (* _r _brightness) (* _g _brightness) (* _b _brightness) _a))
  (`MaterialInstanceDynamic.SetScalarParameterValue` FogSheetMID "MaxOpacity" 3.5)
  (`MaterialInstanceDynamic.SetScalarParameterValue` FogSheetMID "DepthFadeDistance" 1024.0)
  (`MaterialInstanceDynamic.SetScalarParameterValue` FogSheetMID "TilingMaskProjectionDistance" 1024.0)
  (`MaterialInstanceDynamic.SetScalarParameterValue` FogSheetMID "NoiseSize" 200.0)
  (`MaterialInstanceDynamic.SetScalarParameterValue` FogSheetMID "PanningSpeed" 1.0)
  (`MaterialInstanceDynamic.SetScalarParameterValue` FogSheetMID "FadeDistance" 500.0))

(fn `UserConstructionScript`
  (bind _fogsheetmastermaterial (`self.FogSheetMasterMaterial`))
  (bind _returnvalue (`PrimitiveComponent.CreateDynamicMaterialInstance` (`self.StaticMesh1`) 0 _fogsheetmastermaterial "None"))
  (bind _returnvalue_2 (`PrimitiveComponent.CreateDynamicMaterialInstance` (`self.StaticMesh`) 0 _fogsheetmastermaterial "None"))
  (bind _returnvalue_3 (`PrimitiveComponent.CreateDynamicMaterialInstance` (`self.StaticMesh2`) 0 _fogsheetmastermaterial "None"))
  (bind _returnvalue_4 (`PrimitiveComponent.CreateDynamicMaterialInstance` (`self.StaticMesh3`) 0 _fogsheetmastermaterial "None"))
  (`self.ApplyFogSheet` _returnvalue_2)
  (`self.ApplyFogSheet` _returnvalue)
  (`self.ApplyFogSheet` _returnvalue_3)
  (`self.ApplyFogSheet` _returnvalue_4))