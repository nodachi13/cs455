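; Poison skeleton enemy that leaves a poison cloud when its own Die event runs.
; A looping timer turns it toward a random navigable point near the player.
; Hitting Kaelan stuns him and triggers Die, as does hitting anything non-WorldStatic; Die also ragdolls the mesh before delayed destruction.
; Hammer overlaps credit kills and score, then call the parent's Die directly, bypassing this Blueprint's cloud-spawning override.
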(event `Ambulate`
  (bind (_returnvalue_roll _returnvalue_pitch _returnvalue_yaw) (`KismetMathLibrary.BreakRotator` (`KismetMathLibrary.FindLookAtRotation` (`self.K2_GetActorLocation`) (`NavigationSystemV1.K2_GetRandomLocationInNavigableRadius` (`self.K2_GetActorLocation` (`GameplayStatics.GetPlayerCharacter` 0)) 200.0 null null))))
  (`self.K2_SetActorRotation` (`KismetMathLibrary.MakeRotator` 0.0 0.0 _returnvalue_yaw)))

(event `self.ReceiveBeginPlay`
  (`parent.ReceiveBeginPlay`)
  (`KismetSystemLibrary.K2_SetTimerDelegate` (delegate `Ambulate`) 1.5 true))

(event `self.ReceiveTick`
  (params (DeltaSeconds :type "Float (single-precision)"))
  (`parent.ReceiveTick` DeltaSeconds))

(event `self.Die`
  (`|SpawnActorFromClass` "/Game/Blueprints/Skeletons/PoisonCloud.PoisonCloud_C" (`KismetMathLibrary.Conv_VectorToTransform` (`self.K2_GetActorLocation`)) "Undefined" "OverrideRootScale" null null)
  (set `self.Alive` false)
  (`PrimitiveComponent.SetCollisionEnabled` (`self.CapsuleComponent`) "NoCollision")
  (`PrimitiveComponent.SetSimulatePhysics` (`self.Mesh`) true)
  (if (`self.GetPoints`)
    (`self.ProjectPoints`))
  (`KismetSystemLibrary.Delay` 5.0)
  (`self.K2_DestroyActor`))

(event `self.CapsuleComponent.OnComponentBeginOverlap`
  (params (OverlappedComponent :type "PrimitiveComponent Object Reference") (OtherActor :type "Actor Object Reference") (OtherComp :type "PrimitiveComponent Object Reference") (OtherBodyIndex :type Integer) (bFromSweep :type Boolean) (SweepResult :type "HitResult Structure (by ref)"))
  (bind _ashammer (cast `/Game/Blueprints/Hammer` OtherActor))
  (`/Engine/EditorBlueprintResources/StandardMacros.IncrementInt` (`/Game/Blueprints/Hammer.KillCount` _ashammer)
    (:`  `
      (set `/Game/Blueprints/Hammer.KillScore` (+ (`/Game/Blueprints/Hammer.KillScore` _ashammer) (`self.ScoreValue`)) _ashammer)
      (set `self.GetPoints` true)
      (`parent.Die`))))

(event `self.CapsuleComponent.OnComponentHit`
  (params (HitComponent :type "PrimitiveComponent Object Reference") (OtherActor :type "Actor Object Reference") (OtherComp :type "PrimitiveComponent Object Reference") (NormalImpulse :type "Vector Structure") (Hit :type "HitResult Structure (by ref)"))
  (bind _askaelan (cast `/Game/Blueprints/Kaelan` OtherActor)
    (:`then`
      (`/Game/Blueprints/Kaelan.Stun` _askaelan)
      (`self.Die` :!label _label))
    (:`CastFailed`
      (if (`|EnumInequality` (`PrimitiveComponent.GetCollisionObjectType` (`.HitComponent` (`GameplayStatics.BreakHitResult` Hit))) "ECC_WorldStatic")
        (goto _label)))))

(fn `UserConstructionScript`
  (`parent.UserConstructionScript`))