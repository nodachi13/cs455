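; SkelemanThrasher is a skeleton character Blueprint that extends its parent's death behavior and defines a lunging attack.
; Attack snaps the actor to face the target location, then plays a timeline whose curve scales forward movement input each update.
; Attacking is set false at attack start, on timeline finish and on death, and is never set true in this Blueprint.
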(event `self.ReceiveBeginPlay`
  (`parent.ReceiveBeginPlay`))

(event `self.ReceiveTick`
  (params (DeltaSeconds :type "Float (single-precision)")))

(event `self.Die`
  (set `self.Attacking` false)
  (`parent.Die`))

(event `Attack`
  (params (Target :type "Vector Structure"))
  (set `self.Attacking` false)
  (`self.K2_SetActorRotation` (`KismetMathLibrary.FindLookAtRotation` (`self.K2_GetActorLocation`) Target))
  (bind (_direction _newtrack_0) (`Timeline|AttackTimeline`)
    (:`Update`
      (`self.AddMovementInput` (`self.GetActorForwardVector`) _newtrack_0))
    (:`Finished`
      (set `self.Attacking` false))))

(fn `UserConstructionScript`
  (`parent.UserConstructionScript`))