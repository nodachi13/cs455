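; Level director that runs a skeleton wave match in Clear, Survival or Endless mode, tracking kills, score and time.
; Looping timers spawn random skeleton variants at spawn points, with Hardcore spawning faster and normal play unlocking poison and armor types over time.
; Clear wins on a kill target and Survival on elapsed time.
; Finishing kills skeletons, records the mode's best score in the game instance and returns to the main menu.
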(event `self.ReceiveTick`
  (params (DeltaSeconds :type "Float (single-precision)"))
  (bind _output_get (set `self.Time` (+ DeltaSeconds (`self.Time`))))
  (if (and (>= _output_get 180.0) (== (`self.GameMode`) 1))
    (`self.FinishGame` true)))

(event `SpawnSkeletonHardcore`
  (bind _spawnpoints (`self.SpawnPoints`))
  (bind _returnvalue (`self.K2_GetActorLocation` (`|GetArrayItem` _spawnpoints (`KismetMathLibrary.RandomIntegerInRange` 0 (- (`KismetArrayLibrary.Array_Length` _spawnpoints) 1)))))
  (if (`self.Playing`)
    (if (!= (`KismetMathLibrary.RandomIntegerInRange` 0 1) 0)
      (`AIBlueprintHelperLibrary.SpawnAIFromClass` "/Game/Blueprints/Skeletons/SkelemanDefault.SkelemanDefault_C" null _returnvalue)
      (elif (`KismetMathLibrary.RandomBool`)
        (`AIBlueprintHelperLibrary.SpawnAIFromClass` "/Game/Blueprints/Skeletons/SkelemanPoison.SkelemanPoison_C" null _returnvalue)
        (elif (== (`KismetMathLibrary.RandomIntegerInRange` 0 2) 0)
          (`AIBlueprintHelperLibrary.SpawnAIFromClass` "/Game/Blueprints/Skeletons/SkelemanArmor.SkelemanArmor_C" null _returnvalue))))))

(event `self.ReceiveBeginPlay`
  (bind _asnot_amorphous_game_instance (cast `/Game/Blueprints/NotAmorphousGameInstance` (`GameplayStatics.GetGameInstance`)))
  (set `self.GameMode` (`/Game/Blueprints/NotAmorphousGameInstance.GameMode` _asnot_amorphous_game_instance))
  (bind _returnvalue (`|CreateWidget` "/Game/Blueprints/UIStuff/HUD.HUD_C"))
  (bind _output_get (set `self.HUD` _returnvalue))
  (`UserWidget.AddToViewport` _output_get 0)
  (bind _outactors (`GameplayStatics.GetAllActorsOfClass` "/Game/Blueprints/LevelManagement/SkeleSpawnPoint.SkeleSpawnPoint_C"))
  (set `self.SpawnPoints` _outactors)
  (if (`/Game/Blueprints/NotAmorphousGameInstance.Hardcore` _asnot_amorphous_game_instance)
    (`KismetSystemLibrary.K2_SetTimerDelegate` (delegate `SpawnSkeletonHardcore`) 0.6 true)
    (else
      (`KismetSystemLibrary.K2_SetTimerDelegate` (delegate `SpawnSkeleton`) 0.75 true)
      (`KismetSystemLibrary.K2_SetTimerDelegate` (delegate `Begin Poisons`) 20.0)
      (`KismetSystemLibrary.K2_SetTimerDelegate` (delegate `BeginArmors`) 45.0))))

(event `SpawnSkeleton`
  (bind _spawnpoints (`self.SpawnPoints`))
  (bind _returnvalue (`self.K2_GetActorLocation` (`|GetArrayItem` _spawnpoints (`KismetMathLibrary.RandomIntegerInRange` 0 (- (`KismetArrayLibrary.Array_Length` _spawnpoints) 1)))))
  (if (`self.Playing`)
    (if (!= (`KismetMathLibrary.RandomIntegerInRange` 0 2) 0)
      (`AIBlueprintHelperLibrary.SpawnAIFromClass` "/Game/Blueprints/Skeletons/SkelemanDefault.SkelemanDefault_C" null _returnvalue)
      (elif (and (== (`KismetMathLibrary.RandomIntegerInRange` 0 2) 0) (`self.PoisonAllowed`))
        (`AIBlueprintHelperLibrary.SpawnAIFromClass` "/Game/Blueprints/Skeletons/SkelemanPoison.SkelemanPoison_C" null _returnvalue)
        (elif (and (== (`KismetMathLibrary.RandomIntegerInRange` 0 3) 0) (`self.ArmorAllowed`))
          (`AIBlueprintHelperLibrary.SpawnAIFromClass` "/Game/Blueprints/Skeletons/SkelemanArmor.SkelemanArmor_C" null _returnvalue))))))

(event `BeginArmors`
  (set `self.ArmorAllowed` true))

(event `Begin Poisons`
  (set `self.PoisonAllowed` true))

(event `FinishGame`
  (params (Win :type Boolean))
  (bind _score (`self.Score`))
  (if (`self.Playing`)
    (bind _outactors (`GameplayStatics.GetAllActorsOfClass` "/Game/Blueprints/Skeletons/SkelemanDefault.SkelemanDefault_C"))
    (for _array_element _outactors
      (`/Game/Blueprints/Skeletons/SkelemanDefault.Die` _array_element))
    (set `self.Playing` false)
    (if (and (== (`self.GameMode`) 0) (> (`self.Score`) (`/Game/Blueprints/NotAmorphousGameInstance.BestScoreClear` (stale `self.ReceiveBeginPlay` _asnot_amorphous_game_instance))))
      (set `/Game/Blueprints/NotAmorphousGameInstance.BestScoreClear` _score (stale `self.ReceiveBeginPlay` _asnot_amorphous_game_instance))
      (elif (and (== (`self.GameMode`) 1) (> (`self.Score`) (`/Game/Blueprints/NotAmorphousGameInstance.BestScoreSurvival` (stale `self.ReceiveBeginPlay` _asnot_amorphous_game_instance))))
        (set `/Game/Blueprints/NotAmorphousGameInstance.BestScoreSurvival` _score (stale `self.ReceiveBeginPlay` _asnot_amorphous_game_instance))
        (elif (and (== (`self.GameMode`) 2) (> (`self.Score`) (`/Game/Blueprints/NotAmorphousGameInstance.BestScoreEndless` (stale `self.ReceiveBeginPlay` _asnot_amorphous_game_instance))))
          (set `/Game/Blueprints/NotAmorphousGameInstance.BestScoreEndless` _score (stale `self.ReceiveBeginPlay` _asnot_amorphous_game_instance)))))
    (if Win
      (bind _returnvalue (`|CreateWidget` "/Game/Blueprints/UIStuff/VictoryWidget.VictoryWidget_C"))
      (`UserWidget.AddToViewport` _returnvalue 0))
    (`KismetSystemLibrary.Delay` 5.0)
    (`GameplayStatics.OpenLevel` "MainMenu")))

(event `IncreaseKills`
  (params (kills :type Integer))
  (bind _output_get (set `self.Kills` (+ kills (`self.Kills`))))
  (if (and (>= _output_get 200) (== (`self.GameMode`) 0))
    (`self.FinishGame` true)))

(event `IncreaseScore`
  (params (Points :type Integer) (Multiplier :type Integer))
  (set `self.Score` (+ (`self.Score`) (* Points Multiplier))))

(fn `UserConstructionScript`)