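; MainMenuDirector is an actor that populates the main menu scene with a steady stream of spawned AI characters.
; On BeginPlay it gathers all SkeleSpawnPoint actors and calls SpawnSkeles, which starts a short looping timer.
; Each tick of that timer spawns a pawn at a random spawn point, usually a MainMenuSkele and occasionally a MainMenuArmor, with no cap or cleanup in this Blueprint.
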(event `self.ReceiveTick`
  (params (DeltaSeconds :type "Float (single-precision)")))

(event `self.ReceiveBeginPlay`
  (bind _outactors (`GameplayStatics.GetAllActorsOfClass` "/Game/Blueprints/LevelManagement/SkeleSpawnPoint.SkeleSpawnPoint_C"))
  (set `self.SpawnPoints` _outactors)
  (`KismetSystemLibrary.K2_SetTimerDelegate` (delegate `SpawnSkeleton`) 0.6 true))

(event `SpawnSkeleton`
  (bind _spawnpoints (`self.SpawnPoints`))
  (bind _returnvalue (`self.K2_GetActorLocation` (`|GetArrayItem` _spawnpoints (`KismetMathLibrary.RandomIntegerInRange` 0 (- (`KismetArrayLibrary.Array_Length` _spawnpoints) 1)))))
  (if (!= (`KismetMathLibrary.RandomIntegerInRange` 0 4) 0)
    (`AIBlueprintHelperLibrary.SpawnAIFromClass` "/Game/Blueprints/Skeletons/MainMenuSkele.MainMenuSkele_C" null _returnvalue)
    (else
      (`AIBlueprintHelperLibrary.SpawnAIFromClass` "/Game/Blueprints/Skeletons/MainMenuArmor.MainMenuArmor_C" null _returnvalue))))

(fn `UserConstructionScript`)