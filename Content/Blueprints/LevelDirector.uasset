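; LevelDirector is an actor that keeps spawning SkelemanDefault AI pawns at spawn points in the level.
; On BeginPlay it caches all SkeleSpawnPoint actors and starts a short looping timer.
; Each tick of that timer makes a coin flip and, on success, spawns a skeleton at a randomly indexed point.
; The random range includes the array length, so the index can fall out of bounds.
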(event `self.ReceiveBeginPlay`
  (bind _outactors (`GameplayStatics.GetAllActorsOfClass` "/Game/Blueprints/SkeleSpawnPoint.SkeleSpawnPoint_C"))
  (set `self.SpawnPoints` _outactors)
  (`KismetSystemLibrary.K2_SetTimerDelegate` (delegate `SpawnSkeleton`) 0.75 true))

(event `SpawnSkeleton`
  (bind _spawnpoints (`self.SpawnPoints`))
  (if (`KismetMathLibrary.RandomBool`)
    (`AIBlueprintHelperLibrary.SpawnAIFromClass` "/Game/Blueprints/SkelemanDefault.SkelemanDefault_C" null (`self.K2_GetActorLocation` (`|GetArrayItem` _spawnpoints (`KismetMathLibrary.RandomIntegerInRange` 0 (`KismetArrayLibrary.Array_Length` _spawnpoints)))))))

(fn `UserConstructionScript`)