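; SkelemanDefault is a simple enemy character that walks in a straight line until a Hammer kills it.
; On BeginPlay it turns toward a random navigable point around a hard-coded map origin, then adds forward movement every Tick while alive.
; A capsule overlap with a Hammer increments that Hammer's KillCount and triggers Die, which disables capsule collision, ragdolls the mesh and destroys the actor after a delay.
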(event `self.ReceiveTick`
  (params (DeltaSeconds :type "Float (single-precision)"))
  (if (`self.Alive`)
    (`self.AddMovementInput` (`self.GetActorForwardVector`))))

(event `self.ReceiveBeginPlay`
  (bind _output_get (set `self.MapOrigin` (-400.0 41.0 125.0)))
  (`self.K2_SetActorRotation` (`KismetMathLibrary.MakeRotator` 0.0 0.0 (.yaw (`KismetMathLibrary.FindLookAtRotation` (`self.K2_GetActorLocation`) (`NavigationSystemV1.K2_GetRandomLocationInNavigableRadius` _output_get 610.0 null null))))))

(event `self.ReceiveActorBeginOverlap`
  (params (OtherActor :type "Actor Object Reference")))

(event `Die`
  (set `self.Alive` false)
  (`PrimitiveComponent.SetCollisionEnabled` (`self.CapsuleComponent`) "NoCollision")
  (`PrimitiveComponent.SetSimulatePhysics` (`self.Mesh`) true)
  (`KismetSystemLibrary.Delay` 5.0)
  (`self.K2_DestroyActor`))

(event `self.CapsuleComponent.OnComponentBeginOverlap`
  (params (OverlappedComponent :type "PrimitiveComponent Object Reference") (OtherActor :type "Actor Object Reference") (OtherComp :type "PrimitiveComponent Object Reference") (OtherBodyIndex :type Integer) (bFromSweep :type Boolean) (SweepResult :type "HitResult Structure (by ref)"))
  (bind _ashammer (cast `/Game/Blueprints/Hammer` OtherActor))
  (`/Engine/EditorBlueprintResources/StandardMacros.IncrementInt` (`/Game/Blueprints/Hammer.KillCount` _ashammer)
    (:`  `
      (`self.Die`))))

(fn `UserConstructionScript`)